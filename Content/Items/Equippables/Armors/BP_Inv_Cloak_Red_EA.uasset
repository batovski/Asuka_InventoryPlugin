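; BP_Inv_Cloak_Red_EA is the equip actor for a red cloak armor item that raises the Damage value in its owning item's weapon fragment.
; One second after BeginPlay it finds that fragment by tag, increments Damage by one and writes the rebuilt instanced struct back, preserving the other fields.
; Debug prints show the previous damage or flag a failed lookup, which suggests test logic.
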(event `self.ReceiveBeginPlay`
  (bind _returnvalue (`self.GetOwningItem`))
  (`KismetSystemLibrary.Delay` 1.0)
  (`/Engine/EditorBlueprintResources/StandardMacros.IsValid` _returnvalue
    (:`Is Valid`
      (bind (_isfound _returnvalue_2) (`Inv_InventoryStatics.GetFragmentFromItem` _returnvalue (struct :`TagName` "FragmentTags.WeaponFragment")))
      (if _isfound
        (bind _value (`BlueprintInstancedStructLibrary.GetInstancedStructValue` _returnvalue_2)
          (:`Valid`
            (bind (_damage _magazinesize _currentammo) (break `Inv_WeaponFragment` _value))
            (bind (_text_label _value_2 _uielementtag) (break `Inv_WeaponModifier` _damage))
            (`KismetSystemLibrary.PrintString` (`KismetStringLibrary.Conv_DoubleToString` _value_2))
            (bind _returnvalue_3 (`BlueprintInstancedStructLibrary.MakeInstancedStruct` (make `Inv_WeaponFragment` (make `Inv_WeaponModifier` _text_label (+ _value_2 1.0) _uielementtag) _magazinesize _currentammo)))
            (`Inv_InventoryStatics.SetFragmentValuesByTag` _returnvalue _returnvalue_3 (struct :`TagName` "FragmentTags.WeaponFragment")))
          (:`NotValid`
            (`KismetSystemLibrary.PrintString` "2")))
        (else
          (`KismetSystemLibrary.PrintString` "1"))))))

(fn `UserConstructionScript`)